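; Roguelike hero Blueprint that picks up passive items and pills through a sphere overlap.
; Passive items pass their characteristic data and the player character's movement component to AppStatItem.
; Pills apply their own stats to the hero via AppStatPills and are then stored in the MasPill array.
; Debug prints report pickups and walk speed, and the P key prints the collected pill count.
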(event `self.Sphere.OnComponentBeginOverlap`
  (params (OverlappedComponent :type "PrimitiveComponent Object Reference") (OtherActor :type "Actor Object Reference") (OtherComp :type "PrimitiveComponent Object Reference") (OtherBodyIndex :type Integer) (bFromSweep :type Boolean) (SweepResult :type "HitResult Structure (by ref)"))
  (bind _aspassive_item_bp (cast `/Game/Blueprint/Passive_item_BP` OtherActor)
    (:`then`
      (`self.App_stat_item` (`Passive_item.characteristic_passiv_item` _aspassive_item_bp) (`Character.CharacterMovement` (`GameplayStatics.GetPlayerCharacter` 0)))
      (`KismetSystemLibrary.PrintString` "Hello"))
    (:`CastFailed`
      (bind _aspills_bp (cast `/Game/Blueprint/Pills_BP` OtherActor))
      (`Pills.app_stat_pills` _aspills_bp self)
      (`KismetSystemLibrary.PrintString` (`KismetStringLibrary.Conv_NameToString` (`Pills.name` _aspills_bp)))
      (`KismetSystemLibrary.PrintString` (`KismetStringLibrary.Conv_DoubleToString` (`CharacterMovementComponent.MaxWalkSpeed` (`Character.CharacterMovement` (`GameplayStatics.GetPlayerCharacter` 0)))))
      (`KismetArrayLibrary.Array_Add` (`self.Mas_pill`) _aspills_bp))))

(event `Key|P`
  (params (Key :type "Key Structure"))
  (:`Pressed`
    (`KismetSystemLibrary.PrintString` (`KismetStringLibrary.Conv_IntToString` (`KismetArrayLibrary.Array_Length` (`self.Mas_pill`))))))

(fn `UserConstructionScript`)